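; VR player pawn for Pico headsets that manages motion controller actors and a safe-area boundary, with Android Back quitting the game.
; Connect, disconnect and foreground-resume events reset a DoOnce in Tick, deferring RefreshControllerModel to the next tick.
; RefreshControllerModel branches on device type to spawn controllers attached to SceneCameraRoot with input enabled, or destroy stale ones.
; On 6DoF with UseSafeArea, Tick shows MeshSafeArea when the camera nears or exceeds its bounds.
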(event `self.ReceiveTick`
  (params (DeltaSeconds :type "Float (single-precision)"))
  (bind _mesh_safearea (`self.Mesh_SafeArea`))
  (`|ExecutionSequence`
    (:`then_0`
      (bind _is6dof (`PicoBlueprintFunctionLibrary.PicoIs6Dof`))
      ;[1 0.3958 0.3958] Violently update security zones in Tick
      (if _is6dof
        (if (`self.UseSafeArea`)
          (if (>= (`KismetMathLibrary.FMax` (`KismetMathLibrary.Abs` (.x (`SceneComponent.RelativeLocation` (`self.Camera`)))) (`KismetMathLibrary.Abs` (.y (`SceneComponent.RelativeLocation` (`self.Camera`))))) (* (`KismetMathLibrary.FMin` (.x (`SceneComponent.RelativeScale3D` _mesh_safearea)) (.y (`SceneComponent.RelativeScale3D` _mesh_safearea))) 35.0))
            (`SceneComponent.SetVisibility` _mesh_safearea true false)
            (else
              (`SceneComponent.SetVisibility` _mesh_safearea false false))))))
    (:`then_1`
      (`/Engine/EditorBlueprintResources/StandardMacros.DoOnce` true :!label _label
        (:`Completed`
          (`self.RefreshControllerModel`))))))

(event `self.ReceiveBeginPlay`
  (`|ExecutionSequence`
    (:`then_0`
      (`PicoMobileControllerBFlib.PicoSetControllerConnectedStatusChangedDelegate` (delegate `FinchControllerCon`) (delegate `FinchControllerDisC`)))
    (:`then_1`
      (`PicoNeoControllerBPlib.SetControllerConnectedStatusDelegate` (delegate `MainControllerCon`) (delegate `MainControllerDisC`) (delegate `SubControllerCon`) (delegate `SubControllerDisC`)))
    (:`then_2`
      (add `ApplicationLifecycleComponent.ApplicationHasEnteredForegroundDelegate` (`self.ApplicationLifecycle`) (delegate `Resume`)))
    (:`then_3`
      (goto _label :!via `Reset`))))

(event `FinchControllerCon`
  (goto _label :!via `Reset`))

(event `FinchControllerDisC`
  (goto _label :!via `Reset`))

(event `MainControllerCon`
  (goto _label :!via `Reset`))

(event `MainControllerDisC`
  (goto _label :!via `Reset`))

(event `SubControllerCon`
  (goto _label :!via `Reset`))

(event `SubControllerDisC`
  (goto _label :!via `Reset`))

(event `Resume`
  (goto _label :!via `Reset`))

(event `Key|Android_Back`
  (params (Key :type "Key Structure"))
  (:`Pressed`
    (`KismetSystemLibrary.QuitGame` null "Quit" true)))

(fn `RefreshControllerModel`
  (bind _leftcontrollerref (`self.LeftControllerRef`))
  (bind _rightcontrollerref (`self.RightControllerRef`))
  (bind _g1controllerref (`self.G1ControllerRef`))
  (bind _g2controllerref (`self.G2ControllerRef`))
  (bind _leftcontrollerref_2 (`self.LeftControllerRef`))
  (bind _maincontrollerref (`self.MainControllerRef`))
  (bind _subcontrollerref (`self.SubControllerRef`))
  (bind _rightcontrollerref_2 (`self.RightControllerRef`))
  (bind _returnvalue (`PicoMobileControllerBFlib.GetDeviceType`)) ; 0-Unknow, 1-G1, 3-G2
  (switch `int` _returnvalue
    (:`Default`
      ;[1 1 1] SpawnDefaultController
      (bind _returnvalue_2 (`|SpawnActorFromClass` "/PicoMobile/DefaultController.DefaultController_C" (`KismetMathLibrary.MakeTransform` (0.0 0.0 0.0)) "AlwaysSpawn" "OverrideRootScale" self null))
      (bind _output_get (set `self.DefaultController` _returnvalue_2))
      (bind _asplayer_controller (cast `PlayerController` (`self.GetController` self)))
      (`self.EnableInput` _output_get _asplayer_controller)
      (`self.K2_AttachToComponent` _output_get (`self.Scene_CameraRoot`) "None" "SnapToTarget" "SnapToTarget" "KeepRelative" true)
      (`KismetSystemLibrary.PrintString` "buggisme: Spawn DefaultController!"))
    (:`0`
      (`|ExecutionSequence`
        (:`then_0`
          (bind _returnvalue_3 (`PicoNeoControllerBPlib.GetNeoDeviceType`))
          (switch `int` _returnvalue_3
            (:`0`
              (`|ExecutionSequence`
                (:`then_0`
                  (bind _returnvalue_4 (`PicoNeoControllerBPlib.IsMainControllerConnect`))
                  (if _returnvalue_4
                    ;[1 1 1] If the main handle is connected, but there is no main handle, instance it.
                    (if (== null (`self.MainControllerRef`))
                      (bind _returnvalue_5 (`|SpawnActorFromClass` "/PicoNeoController/CV/MainController.MainController_C" (`KismetMathLibrary.MakeTransform` (0.0 0.0 0.0)) "AlwaysSpawn" "OverrideRootScale" self null))
                      (bind _output_get_2 (set `self.MainControllerRef` _returnvalue_5))
                      (bind _asplayer_controller_2 (cast `PlayerController` (`self.GetController` self)))
                      (`self.EnableInput` _output_get_2 _asplayer_controller_2)
                      (`self.K2_AttachToComponent` _output_get_2 (`self.Scene_CameraRoot`) "None" "SnapToTarget" "SnapToTarget" "KeepRelative" true)
                      (`KismetSystemLibrary.PrintString` "buggisme: Spawn main controller!"))
                    (else
                      ;[1 1 1] If the main handle is disconnected, but there is main handle, destroy it.
                      (if (not (== null _maincontrollerref))
                        (`self.K2_DestroyActor` _maincontrollerref)
                        (set `self.MainControllerRef` null)
                        (`KismetSystemLibrary.PrintString` "buggisme: Destroy main controller")))))
                (:`then_1`
                  (bind _returnvalue_6 (`PicoNeoControllerBPlib.IsSubControllerConnect`))
                  (if _returnvalue_6
                    ;[1 1 1] If the sub handle is connected, but there is no sub handle, instance it.
                    (if (== null (`self.SubControllerRef`))
                      (bind _returnvalue_7 (`|SpawnActorFromClass` "/PicoNeoController/CV/SubController.SubController_C" (`KismetMathLibrary.MakeTransform` (0.0 0.0 0.0)) "AlwaysSpawn" "OverrideRootScale" self null))
                      (bind _output_get_3 (set `self.SubControllerRef` _returnvalue_7))
                      (bind _asplayer_controller_3 (cast `PlayerController` (`self.GetController` self)))
                      (`self.EnableInput` _output_get_3 _asplayer_controller_3)
                      (`self.K2_AttachToComponent` _output_get_3 (`self.Scene_CameraRoot`) "None" "SnapToTarget" "SnapToTarget" "KeepRelative" true)
                      (`KismetSystemLibrary.PrintString` "buggisme: Spawn sub Controller!"))
                    (else
                      ;[1 1 1] If the sub handle is disconnected, but there is sub handle, destroy it.
                      (if (not (== null _subcontrollerref))
                        (`self.K2_DestroyActor` _subcontrollerref)
                        (set `self.SubControllerRef` null)
                        (`KismetSystemLibrary.PrintString` "buggisme: Destroy sub controllert!")))))))
            (:`4`
              (`|ExecutionSequence`
                (:`then_0`
                  (bind _returnvalue_8 (`PicoNeoControllerBPlib.IsMainControllerConnect`))
                  (if _returnvalue_8
                    ;[1 1 1] If the left handle is connected, but there is no left handle, instance it.
                    (if (== null _leftcontrollerref)
                      (bind _returnvalue_9 (`|SpawnActorFromClass` "/PicoNeoController/CV2/LeftController.LeftController_C" (`KismetMathLibrary.MakeTransform` (0.0 0.0 0.0)) "AlwaysSpawn" "OverrideRootScale" self null))
                      (bind _output_get_4 (set `self.LeftControllerRef` _returnvalue_9))
                      (bind _asplayer_controller_4 (cast `PlayerController` (`self.GetController` self)))
                      (`self.EnableInput` _output_get_4 _asplayer_controller_4)
                      (`self.K2_AttachToComponent` _output_get_4 (`self.Scene_CameraRoot`) "None" "SnapToTarget" "SnapToTarget" "KeepRelative" true)
                      (`KismetSystemLibrary.PrintString` "buggisme: Spawn left controller!")
                      (else
                        (`/PicoNeoController/CV2/LeftController.RefreshMeshRayLeft` _leftcontrollerref)))
                    (else
                      ;[1 1 1] If the left handle is disconnected, but there is left handle, destroy it.
                      (if (not (== null _leftcontrollerref_2))
                        (`self.K2_DestroyActor` _leftcontrollerref_2)
                        (set `self.LeftControllerRef` null)
                        (`KismetSystemLibrary.PrintString` "buggisme: Destroy left controller")))))
                (:`then_1`
                  (bind _returnvalue_10 (`PicoNeoControllerBPlib.IsSubControllerConnect`))
                  (if _returnvalue_10
                    ;[1 1 1] If the right handle is connected, but there is no right handle, instance it.
                    (if (== null _rightcontrollerref_2)
                      (bind _returnvalue_11 (`|SpawnActorFromClass` "/PicoNeoController/CV2/RightController.RightController_C" (`KismetMathLibrary.MakeTransform` (0.0 0.0 0.0)) "AlwaysSpawn" "OverrideRootScale" self null))
                      (bind _output_get_5 (set `self.RightControllerRef` _returnvalue_11))
                      (bind _asplayer_controller_5 (cast `PlayerController` (`self.GetController` self)))
                      (`self.EnableInput` _output_get_5 _asplayer_controller_5)
                      (`self.K2_AttachToComponent` _output_get_5 (`self.Scene_CameraRoot`) "None" "SnapToTarget" "SnapToTarget" "KeepRelative" true)
                      (`KismetSystemLibrary.PrintString` "buggisme: Spawn right controller!")
                      (else
                        (`/PicoNeoController/CV2/RightController.RefreshMeshRayRight` _rightcontrollerref_2)))
                    (else
                      ;[1 1 1] If the right handle is disconnected, but there is right handle, destroy it.
                      (if (not (== null _rightcontrollerref))
                        (`self.K2_DestroyActor` _rightcontrollerref)
                        (set `self.RightControllerRef` null)
                        (`KismetSystemLibrary.PrintString` "buggisme: Destroy right controller")))))))))
        (:`then_1`
          ;[1 1 1] If GetDeviceType is 0, it is possible to run on G1/2 but not with the handle. If there is a handle instance to destroy it
          (`|ExecutionSequence`
            (:`then_0`
              (if (!= _g1controllerref null)
                (`self.K2_DestroyActor` _g1controllerref)
                (set `self.G1ControllerRef` null)
                (`KismetSystemLibrary.PrintString` "buggisme: Destroy G1 controllert!")))
            (:`then_1`
              (if (!= _g2controllerref null)
                (`self.K2_DestroyActor` _g2controllerref)
                (set `self.G2ControllerRef` null)
                (`KismetSystemLibrary.PrintString` "buggisme: Destroy G2 controllert!")))))))
    (:`1`
      ;[1 1 1] If the G1 handle is connected, but there is no G1 handle, instance it.
      (if (== null (`self.G1ControllerRef`))
        (bind _returnvalue_12 (`|SpawnActorFromClass` "/PicoMobileController/G1/G1Controller.G1Controller_C" (`KismetMathLibrary.MakeTransform` (0.0 0.0 0.0)) "AlwaysSpawn" "OverrideRootScale" self null))
        (bind _output_get_6 (set `self.G1ControllerRef` _returnvalue_12))
        (bind _asplayer_controller_6 (cast `PlayerController` (`self.GetController` self)))
        (`self.EnableInput` _output_get_6 _asplayer_controller_6)
        (`self.K2_AttachToComponent` _output_get_6 (`self.Scene_CameraRoot`) "None" "SnapToTarget" "SnapToTarget" "KeepRelative" true)
        (`KismetSystemLibrary.PrintString` "buggisme: Spawn G1controller!")))
    (:`3`
      ;[1 1 1] If the G2 handle is connected, but there is no G2 handle, instance it.
      (if (== null (`self.G2ControllerRef`))
        (bind _returnvalue_13 (`|SpawnActorFromClass` "/PicoMobileController/G2/G2Controller.G2Controller_C" (`KismetMathLibrary.MakeTransform` (0.0 0.0 0.0)) "AlwaysSpawn" "OverrideRootScale" self null))
        (bind _output_get_7 (set `self.G2ControllerRef` _returnvalue_13))
        (bind _asplayer_controller_7 (cast `PlayerController` (`self.GetController` self)))
        (`self.EnableInput` _output_get_7 _asplayer_controller_7)
        (`self.K2_AttachToComponent` _output_get_7 (`self.Scene_CameraRoot`) "None" "SnapToTarget" "SnapToTarget" "KeepRelative" true)
        (`KismetSystemLibrary.PrintString` "buggisme: Spawn G2 controller!")))))

(fn `UserConstructionScript`)