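; TraceInteractionInterface is a Blueprint interface for objects in the VR room that respond to trace-based interaction.
; It declares callbacks for a trace entering or leaving an object or a specific component, moving across it, and activation press and release.
; Each function receives the hit result, with the component or instigator where relevant, and returns a boolean that defaults to false.
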(fn `TraceActivateDown`
  (params (Hit :type "HitResult Structure") (Instigator :type "Actor Object Reference"))
  (returns (Return :type Boolean))
  (return false))

(fn `TraceActivateUp`
  (params (Hit :type "HitResult Structure") (Instigator :type "Actor Object Reference"))
  (returns (Return :type Boolean))
  (return false))

(fn `TraceHitComponent`
  (params (Hit :type "HitResult Structure") (Component :type "PrimitiveComponent Object Reference"))
  (returns (Return :type Boolean))
  (return false))

(fn `TraceHitObject`
  (params (Hit :type "HitResult Structure"))
  (returns (Return :type Boolean))
  (return false))

(fn `TraceLeaveComponent`
  (params (Hit :type "HitResult Structure") (Component :type "PrimitiveComponent Object Reference"))
  (returns (Return :type Boolean))
  (return false))

(fn `TraceLeaveObject`
  (params (Hit :type "HitResult Structure"))
  (returns (Return :type Boolean))
  (return false))

(fn `TraceMove`
  (params (Hit :type "HitResult Structure (by ref)"))
  (returns (Return :type Boolean))
  (return false))